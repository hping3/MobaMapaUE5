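; Configurable prefab Blueprint that assembles a medieval castle keep from static mesh components in its construction script.
; The Interior flag picks one of two base meshes, and Huts adds up to two hut meshes high on the keep.
; Towers fills up to four corners through cascading count checks, while TowerType selects among three tower variants, each stacking three pieces at fixed offsets.
; The event graph has no active logic.
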(event EventBeginPlay)

(event Collision|EventActorBeginOverlap
  (params (OtherActor :type Actor%20Object%20Reference)))

(event EventTick
  (params (DeltaSeconds :type Float%20%28single-precision%29)))

(fn ConstructionScript
  (bind _towers (Variables|Default|GetTowers))
  (bind _returnvalue (>= _towers 4))
  (bind _returnvalue_2 (>= _towers 2))
  (bind _returnvalue_3 (>= _towers 3))
  (if (Variables|Default|GetInterior)
    (AddComponent|AddStaticMeshComponent false)
    (else
      (AddComponent|AddStaticMeshComponent false)))
  ;[1 1 1] Huts
  (switch int (Variables|Default|GetHuts)
    (:0
      _)
    (:1
      (AddComponent|AddStaticMeshComponent false (Math|Transform|MakeTransform "0.000000,500.000000,3600.000000" "0,90.000000, 0")))
    (:2
      (AddComponent|AddStaticMeshComponent false (Math|Transform|MakeTransform "0.000000,500.000000,3600.000000" "0,90.000000, 0"))
      (AddComponent|AddStaticMeshComponent false (Math|Transform|MakeTransform "0.000000,-500.000000,3600.000000" "0,90.000000, 0"))))
  ;[1 1 1] If the tower amount is set to 0, don't perform any logic.
  (if (not (== _towers 0))
    (switch int (Variables|Default|GetTowerType)
      (:1
        ;[1 1 1] If tower amount is above one, proceed with spawning a tower
        (if (>= _towers 1)
          (AddComponent|AddStaticMeshComponent false (Math|Transform|MakeTransform "2300.000000,2300.000000,0.000000"))
          (AddComponent|AddStaticMeshComponent false (Math|Transform|MakeTransform "2300.000000,2300.000000,1180.000000"))
          (AddComponent|AddStaticMeshComponent false (Math|Transform|MakeTransform "2300.000000,2300.000000,2600.000000"))
          ;[1 1 1] If tower amount is above two, proceed with spawning a 2nd tower etc
          (if _returnvalue_2
            (AddComponent|AddStaticMeshComponent false (Math|Transform|MakeTransform "-2300.000000,2300.000000,0.000000"))
            (AddComponent|AddStaticMeshComponent false (Math|Transform|MakeTransform "-2300.000000,2300.000000,1180.000000"))
            (AddComponent|AddStaticMeshComponent false (Math|Transform|MakeTransform "-2300.000000,2300.000000,2600.000000"))
            (if _returnvalue_3
              (AddComponent|AddStaticMeshComponent false (Math|Transform|MakeTransform "2300.000000,-2300.000000,0.000000"))
              (AddComponent|AddStaticMeshComponent false (Math|Transform|MakeTransform "2300.000000,-2300.000000,1180.000000"))
              (AddComponent|AddStaticMeshComponent false (Math|Transform|MakeTransform "2300.000000,-2300.000000,2600.000000"))
              (if _returnvalue
                (AddComponent|AddStaticMeshComponent false (Math|Transform|MakeTransform "-2300.000000,-2300.000000,0.000000"))
                (AddComponent|AddStaticMeshComponent false (Math|Transform|MakeTransform "-2300.000000,-2300.000000,1180.000000"))
                (AddComponent|AddStaticMeshComponent false (Math|Transform|MakeTransform "-2300.000000,-2300.000000,2600.000000")))))))
      (:2
        (AddComponent|AddStaticMeshComponent false (Math|Transform|MakeTransform "2300.000000,2300.000000,0.000000"))
        (AddComponent|AddStaticMeshComponent false (Math|Transform|MakeTransform "2300.000000,2300.000000,2200.000000"))
        (AddComponent|AddStaticMeshComponent false (Math|Transform|MakeTransform "2300.000000,2300.000000,4400.000000"))
        (if _returnvalue_2
          (AddComponent|AddStaticMeshComponent false (Math|Transform|MakeTransform "-2300.000000,2300.000000,0.000000"))
          (AddComponent|AddStaticMeshComponent false (Math|Transform|MakeTransform "-2300.000000,2300.000000,2200.000000"))
          (AddComponent|AddStaticMeshComponent false (Math|Transform|MakeTransform "-2300.000000,2300.000000,4400.000000"))
          (if _returnvalue_3
            (AddComponent|AddStaticMeshComponent false (Math|Transform|MakeTransform "2300.000000,-2300.000000,0.000000"))
            (AddComponent|AddStaticMeshComponent false (Math|Transform|MakeTransform "2300.000000,-2300.000000,2200.000000"))
            (AddComponent|AddStaticMeshComponent false (Math|Transform|MakeTransform "2300.000000,-2300.000000,4400.000000"))
            (if _returnvalue
              (AddComponent|AddStaticMeshComponent false (Math|Transform|MakeTransform "-2300.000000,-2300.000000,0.000000"))
              (AddComponent|AddStaticMeshComponent false (Math|Transform|MakeTransform "-2300.000000,-2300.000000,2200.000000"))
              (AddComponent|AddStaticMeshComponent false (Math|Transform|MakeTransform "-2300.000000,-2300.000000,4400.000000"))))))
      (:3
        (AddComponent|AddStaticMeshComponent false (Math|Transform|MakeTransform "2300.000000,2300.000000,0.000000"))
        (AddComponent|AddStaticMeshComponent false (Math|Transform|MakeTransform "2300.000000,2300.000000,2200.000000"))
        (AddComponent|AddStaticMeshComponent false (Math|Transform|MakeTransform "2300.000000,2300.000000,4400.000000"))
        (if _returnvalue_2
          (AddComponent|AddStaticMeshComponent false (Math|Transform|MakeTransform "-2300.000000,2300.000000,0.000000"))
          (AddComponent|AddStaticMeshComponent false (Math|Transform|MakeTransform "-2300.000000,2300.000000,2200.000000"))
          (AddComponent|AddStaticMeshComponent false (Math|Transform|MakeTransform "-2300.000000,2300.000000,4400.000000"))
          (if _returnvalue_3
            (AddComponent|AddStaticMeshComponent false (Math|Transform|MakeTransform "2300.000000,-2300.000000,0.000000"))
            (AddComponent|AddStaticMeshComponent false (Math|Transform|MakeTransform "2300.000000,-2300.000000,2200.000000"))
            (AddComponent|AddStaticMeshComponent false (Math|Transform|MakeTransform "2300.000000,-2300.000000,4400.000000"))
            (if _returnvalue
              (AddComponent|AddStaticMeshComponent false (Math|Transform|MakeTransform "-2300.000000,-2300.000000,0.000000"))
              (AddComponent|AddStaticMeshComponent false (Math|Transform|MakeTransform "-2300.000000,-2300.000000,2200.000000"))
              (AddComponent|AddStaticMeshComponent false (Math|Transform|MakeTransform "-2300.000000,-2300.000000,4400.000000")))))))))