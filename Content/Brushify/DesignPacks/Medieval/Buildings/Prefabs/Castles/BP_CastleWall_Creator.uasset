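; Castle wall builder that lays palisade or stone-wall meshes along an editable spline in the Construction Script.
; It splits the spline by SectionLength into spline mesh segments with clamped tangents and a slight end overlap, choosing Palisade or a WallHeight variant.
; With Towers enabled, a DoN capped at the point count uses the segment index to place two stacked instanced-mesh pieces at spline points, selected by TowerVariation.
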(event EventBeginPlay)

(event Collision|EventActorBeginOverlap
  (params (OtherActor :type Actor%20Object%20Reference)))

(event EventTick
  (params (DeltaSeconds :type Float%20%28single-precision%29)))

(fn ConstructionScript
  (bind _spline (Variables|Default|GetSpline))
  (bind _spline_2 (Variables|Default|GetSpline))
  (for _index (range 0 (- (Math|Float|Truncate (/ (Spline|GetSplineLength _spline) (Variables|Default|GetSectionLength))) 1))
    (if (Variables|Default|GetPalisade)
      (bind _returnvalue (AddComponent|AddSplineMeshComponent false))
      (else
        (switch int (Variables|Default|GetWallHeight)
          (:1
            (bind _returnvalue_2 (AddComponent|AddSplineMeshComponent false)))
          (:2
            (bind _returnvalue_3 (AddComponent|AddSplineMeshComponent false (Math|Transform|MakeTransform "0, 0, 0")))))))
    (SplineMesh|SetStartandEnd _returnvalue_3 (Spline|GetLocationatDistanceAlongSpline _spline_2 (* (+ _index 0) (Variables|Default|GetSectionLength)) "Local") (Math|Vector|ClampVectorSize (Spline|GetTangentatDistanceAlongSpline _spline_2 (* (+ _index 0) (Variables|Default|GetSectionLength)) "Local") 0.0 (Variables|Default|GetSectionLength)) (Spline|GetLocationatDistanceAlongSpline _spline_2 (+ (* (+ _index 1) (Variables|Default|GetSectionLength)) 1e+01) "Local") (Math|Vector|ClampVectorSize (Spline|GetTangentatDistanceAlongSpline _spline_2 (+ (* (+ _index 1) (Variables|Default|GetSectionLength)) 1e+01) "Local") 0.0 (Variables|Default|GetSectionLength)) true :!class /Script/Engine.SplineMeshComponent)
    (if (Variables|Default|GetTowers)
      (Utilities|FlowControl|DoN (Spline|GetNumberOfSplinePoints (Variables|Default|GetSpline))
        (:Exit
          (switch int (Variables|Default|GetTowerVariation)
            (:1
              (AddComponent|AddInstancedStaticMeshComponent false (Math|Transform|MakeTransform (.Location (Math|Transform|BreakTransform (Spline|GetTransformatSplinePoint _spline (- _index 0) "Local" false)))))
              (AddComponent|AddInstancedStaticMeshComponent false (Math|Transform|MakeTransform (+ (.Location (Math|Transform|BreakTransform (Spline|GetTransformatSplinePoint _spline (- _index 0) "Local" false))) "0,0.000000,2406.000000") "0, 0, 0" (.Scale (Math|Transform|BreakTransform (Spline|GetTransformatSplinePoint _spline (- _index 0) "Local" false))))))
            (:2
              (AddComponent|AddInstancedStaticMeshComponent false (Math|Transform|MakeTransform (.Location (Math|Transform|BreakTransform (Spline|GetTransformatSplinePoint _spline (- _index 0) "Local" false)))))
              (AddComponent|AddInstancedStaticMeshComponent false (Math|Transform|MakeTransform (+ (.Location (Math|Transform|BreakTransform (Spline|GetTransformatSplinePoint _spline (- _index 0) "Local" false))) "0,0.000000,2406.000000") "0, 0, 0" (.Scale (Math|Transform|BreakTransform (Spline|GetTransformatSplinePoint _spline (- _index 0) "Local" false))))))
            (:3
              (AddComponent|AddInstancedStaticMeshComponent false (Math|Transform|MakeTransform (.Location (Math|Transform|BreakTransform (Spline|GetTransformatSplinePoint _spline (- _index 0) "Local" false)))))
              (AddComponent|AddInstancedStaticMeshComponent false (Math|Transform|MakeTransform (+ (.Location (Math|Transform|BreakTransform (Spline|GetTransformatSplinePoint _spline (- _index 0) "Local" false))) "0,0.000000,2406.000000") "0, 0, 0" (.Scale (Math|Transform|BreakTransform (Spline|GetTransformatSplinePoint _spline (- _index 0) "Local" false))))))
            (:4
              (AddComponent|AddInstancedStaticMeshComponent false (Math|Transform|MakeTransform (.Location (Math|Transform|BreakTransform (Spline|GetTransformatSplinePoint _spline (- _index 0) "Local" false)))))
              (AddComponent|AddInstancedStaticMeshComponent false (Math|Transform|MakeTransform (+ (.Location (Math|Transform|BreakTransform (Spline|GetTransformatSplinePoint _spline (- _index 0) "Local" false))) "0,0.000000,1180.000000") "0, 0, 0" (.Scale (Math|Transform|BreakTransform (Spline|GetTransformatSplinePoint _spline (- _index 0) "Local" false))))))))))))