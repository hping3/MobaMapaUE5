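; Castle tower prefab that assembles a medieval tower from stacked static mesh components in its Construction Script.
; TowerType selects one of three variants, and TowerHeight drives nested branches that add pieces at hard-coded vertical offsets above a base.
; The first two variants share a layout with slightly narrowed middle sections, while the third stays full width and supports fewer height levels.
; The event graph has no active logic.
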(event EventBeginPlay)

(event Collision|EventActorBeginOverlap
  (params (OtherActor :type Actor%20Object%20Reference)))

(event EventTick
  (params (DeltaSeconds :type Float%20%28single-precision%29)))

(fn ConstructionScript
  (switch int (Variables|Default|GetTowerType)
    (:1
      (AddComponent|AddStaticMeshComponent false (Math|Transform|MakeTransform "0, 0, 0"))
      (if (>= (Variables|Default|GetTowerHeight) 1)
        (if (>= (Variables|Default|GetTowerHeight) 2)
          (if (>= (Variables|Default|GetTowerHeight) 3)
            (if (>= (Variables|Default|GetTowerHeight) 4)
              (AddComponent|AddStaticMeshComponent false (Math|Transform|MakeTransform "0.000000,0.000000,1180.000000" "0, 0, 0" "0.900000,0.900000,1"))
              (AddComponent|AddStaticMeshComponent false (Math|Transform|MakeTransform "0.000000,0.000000,2400.000000" "0, 0, 0" "0.900000,0.900000,1.000000"))
              (AddComponent|AddStaticMeshComponent false (Math|Transform|MakeTransform "0.000000,0.000000,3600.000000" "0, 0, 0" "0.900000,0.900000,1"))
              (AddComponent|AddStaticMeshComponent false (Math|Transform|MakeTransform "0.000000,0.000000,4800.000000" "0, 0, 0" "0.900000,0.900000,1"))
              (AddComponent|AddStaticMeshComponent false (Math|Transform|MakeTransform "0.000000,0.000000,6000.000000"))
              (else
                (AddComponent|AddStaticMeshComponent false (Math|Transform|MakeTransform "0.000000,0.000000,1180.000000" "0, 0, 0" "0.900000,0.900000,1"))
                (AddComponent|AddStaticMeshComponent false (Math|Transform|MakeTransform "0.000000,0.000000,2400.000000" "0, 0, 0" "0.900000,0.900000,1"))
                (AddComponent|AddStaticMeshComponent false (Math|Transform|MakeTransform "0.000000,0.000000,3600.000000" "0, 0, 0" "0.900000,0.900000,1"))
                (AddComponent|AddStaticMeshComponent false (Math|Transform|MakeTransform "0.000000,0.000000,4800.000000"))))
            (else
              (AddComponent|AddStaticMeshComponent false (Math|Transform|MakeTransform "0.000000,0.000000,1180.000000" "0, 0, 0" "0.900000,0.900000,1"))
              (AddComponent|AddStaticMeshComponent false (Math|Transform|MakeTransform "0.000000,0.000000,2400.000000" "0, 0, 0" "0.900000,0.900000,1"))
              (AddComponent|AddStaticMeshComponent false (Math|Transform|MakeTransform "0.000000,0.000000,3600.000000"))))
          (else
            (AddComponent|AddStaticMeshComponent false (Math|Transform|MakeTransform "0.000000,0.000000,1180.000000" "0, 0, 0" "0.900000,0.900000,1"))
            (AddComponent|AddStaticMeshComponent false (Math|Transform|MakeTransform "0.000000,0.000000,2400.000000"))))
        (else
          (AddComponent|AddStaticMeshComponent false (Math|Transform|MakeTransform "0.000000,0.000000,1200.000000")))))
    (:2
      (AddComponent|AddStaticMeshComponent false (Math|Transform|MakeTransform "0, 0, 0"))
      (if (>= (Variables|Default|GetTowerHeight) 1)
        (if (>= (Variables|Default|GetTowerHeight) 2)
          (if (>= (Variables|Default|GetTowerHeight) 3)
            (if (>= (Variables|Default|GetTowerHeight) 4)
              (AddComponent|AddStaticMeshComponent false (Math|Transform|MakeTransform "0.000000,0.000000,1180.000000" "0, 0, 0" "0.900000,0.900000,1"))
              (AddComponent|AddStaticMeshComponent false (Math|Transform|MakeTransform "0.000000,0.000000,2400.000000" "0, 0, 0" "0.900000,0.900000,1.000000"))
              (AddComponent|AddStaticMeshComponent false (Math|Transform|MakeTransform "0.000000,0.000000,3600.000000" "0, 0, 0" "0.900000,0.900000,1"))
              (AddComponent|AddStaticMeshComponent false (Math|Transform|MakeTransform "0.000000,0.000000,4800.000000" "0, 0, 0" "0.900000,0.900000,1"))
              (AddComponent|AddStaticMeshComponent false (Math|Transform|MakeTransform "0.000000,0.000000,6000.000000"))
              (else
                (AddComponent|AddStaticMeshComponent false (Math|Transform|MakeTransform "0.000000,0.000000,1180.000000" "0, 0, 0" "0.900000,0.900000,1"))
                (AddComponent|AddStaticMeshComponent false (Math|Transform|MakeTransform "0.000000,0.000000,2400.000000" "0, 0, 0" "0.900000,0.900000,1.000000"))
                (AddComponent|AddStaticMeshComponent false (Math|Transform|MakeTransform "0.000000,0.000000,3600.000000" "0, 0, 0" "0.900000,0.900000,1"))
                (AddComponent|AddStaticMeshComponent false (Math|Transform|MakeTransform "0.000000,0.000000,4800.000000"))))
            (else
              (AddComponent|AddStaticMeshComponent false (Math|Transform|MakeTransform "0.000000,0.000000,1180.000000" "0, 0, 0" "0.900000,0.900000,1"))
              (AddComponent|AddStaticMeshComponent false (Math|Transform|MakeTransform "0.000000,0.000000,2400.000000" "0, 0, 0" "0.900000,0.900000,1"))
              (AddComponent|AddStaticMeshComponent false (Math|Transform|MakeTransform "0.000000,0.000000,3600.000000"))))
          (else
            (AddComponent|AddStaticMeshComponent false (Math|Transform|MakeTransform "0.000000,0.000000,1180.000000" "0, 0, 0" "0.900000,0.900000,1"))
            (AddComponent|AddStaticMeshComponent false (Math|Transform|MakeTransform "0.000000,0.000000,2400.000000"))))
        (else
          (AddComponent|AddStaticMeshComponent false (Math|Transform|MakeTransform "0.000000,0.000000,1200.000000")))))
    (:3
      (AddComponent|AddStaticMeshComponent false (Math|Transform|MakeTransform "0, 0, 0"))
      (if (>= (Variables|Default|GetTowerHeight) 1)
        (if (>= (Variables|Default|GetTowerHeight) 2)
          (AddComponent|AddStaticMeshComponent false (Math|Transform|MakeTransform "0.000000,0.000000,1180.000000"))
          (AddComponent|AddStaticMeshComponent false (Math|Transform|MakeTransform "0.000000,0.000000,2600.000000"))
          (AddComponent|AddStaticMeshComponent false (Math|Transform|MakeTransform "0.000000,0.000000,4000.000000"))
          (else
            (AddComponent|AddStaticMeshComponent false (Math|Transform|MakeTransform "0.000000,0.000000,1180.000000"))
            (AddComponent|AddStaticMeshComponent false (Math|Transform|MakeTransform "0.000000,0.000000,2600.000000"))))
        (else
          (AddComponent|AddStaticMeshComponent false (Math|Transform|MakeTransform "0.000000,0.000000,1200.000000")))))))