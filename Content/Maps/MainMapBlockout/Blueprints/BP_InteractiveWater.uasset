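; Interactive water surface actor that sets up a render-target ripple simulation driven by the player's mesh.
; An underwater box adds overlapping player meshes to an orthographic scene capture, which follows the captured player in XY on Tick.
; BeginPlay creates height, normal and capture targets plus height, normal and splat materials, wiring captures into splat and normals into water.
; The simulation draw passes are absent from these graphs.
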(event OnComponentBeginOverlap(Box)
  (params (OverlappedComponent :type Primitive%20Component%20Object%20Reference) (OtherActor :type Actor%20Object%20Reference) (OtherComp :type Primitive%20Component%20Object%20Reference) (OtherBodyIndex :type Integer) (bFromSweep :type Boolean) (SweepResult :type Hit%20Result%20Structure%20%28by%20ref%29))
  (bind _asthird_person_character (Utilities|Casting|CastTo OtherActor))
  (Variables|Default|SetCapturedPlayer 0 _asthird_person_character)
  (Rendering|SceneCapture|ShowOnlyComponent (Variables|Default|GetSceneCaptureComponent2D) (Variables|/Script/Engine.Character|GetMesh (.CapturedPlayer (Variables|Default|GetCapturedPlayer)))))

(event OnComponentEndOverlap(Box)
  (params (OverlappedComponent :type Primitive%20Component%20Object%20Reference) (OtherActor :type Actor%20Object%20Reference) (OtherComp :type Primitive%20Component%20Object%20Reference) (OtherBodyIndex :type Integer))
  (if (== OtherActor (.CapturedPlayer (Variables|Default|GetCapturedPlayer)))
    (Class|SceneCaptureComponent|RemoveShowOnlyComponent (Variables|Default|GetSceneCaptureComponent2D) (Variables|/Script/Engine.Character|GetMesh (.CapturedPlayer (Variables|Default|GetCapturedPlayer))))
    (Variables|Default|SetCapturedPlayer 0)))

(event EventBeginPlay
  (CallFunction|PrepareHeightRT (Variables|Default|GetRenderTargetResolution))
  (bind _returnvalue (Rendering|Material|CreateDynamicMaterialInstance "/MobaMapContent/Maps/MainMapBlockout/Materials/M_HeightSimulation.M_HeightSimulation" "None" "None" :!class /Script/Engine.KismetMaterialLibrary))
  (Variables|Default|SetMID_HeightSimulation _returnvalue)
  (bind _returnvalue_2 (Rendering|Material|CreateDynamicMaterialInstance "/MobaMapContent/Maps/MainMapBlockout/Materials/M_ComputeNormals.M_ComputeNormals" "None" "None" :!class /Script/Engine.KismetMaterialLibrary))
  (Variables|Default|SetMID_ComputeNormals _returnvalue_2)
  (bind _returnvalue_3 (Rendering|Material|CreateDynamicMaterialInstance "/MobaMapContent/Maps/MainMapBlockout/Materials/M_Splat.M_Splat" "None" "None" :!class /Script/Engine.KismetMaterialLibrary))
  (Variables|Default|SetMID_Splat _returnvalue_3)
  (CallFunction|PrepareCaptureRT (Variables|Default|GetSceneCaptureResolution))
  (CallFunction|PrepareSceneCapture)
  (CallFunction|PrepareBaseWater)
  (if (Collision|IsOverlappingActor (Game|GetPlayerCharacter 0) :!class /Script/Engine.Actor)
    (bind _asthird_person_character (Utilities|Casting|CastTo (Game|GetPlayerCharacter 0)))
    (Variables|Default|SetCapturedPlayer 0 _asthird_person_character)
    (Rendering|SceneCapture|ShowOnlyComponent (Variables|Default|GetSceneCaptureComponent2D) (Variables|/Script/Engine.Character|GetMesh (.CapturedPlayer (Variables|Default|GetCapturedPlayer))))))

(event Collision|EventActorBeginOverlap
  (params (OtherActor :type Actor%20Object%20Reference)))

(event EventTick
  (params (DeltaSeconds :type Float%20%28single-precision%29))
  (bind _capturedplayer (Variables|Default|GetCapturedPlayer))
  (bind _returnvalue (Transformation|GetActorLocation _capturedplayer))
  (Utilities|IsValid (.CapturedPlayer (Variables|Default|GetCapturedPlayer))
    (:Is%20Valid
      (Transformation|SetWorldLocation (Variables|Default|GetSceneCaptureComponent2D) (Math|Vector|MakeVector (.x _returnvalue) (.y _returnvalue) (.z (Transformation|GetWorldLocation (Variables|Default|GetSceneCaptureComponent2D)))) false false))))

(fn ConstructionScript
  (bind _endpoint (Variables|Default|GetEndPoint))
  (bind _returnvalue (/ _endpoint 1e+02))
  (Transformation|SetWorldScale3D (Variables|Default|GetStaticMesh) (Math|Vector|MakeVector (.x _returnvalue) (.y _returnvalue) 1.0))
  (Transformation|SetRelativeScale3D (Variables|Default|GetBox) (Math|Vector|MakeVector 1.0 1.0 (Variables|Default|GetUnderWaterHeight)))
  (Transformation|SetRelativeLocation (Variables|Default|GetBox) (Math|Vector|MakeVector 0.0 0.0 (* (Variables|Default|GetUnderWaterHeight) -1.0)) false false)
  (bind _returnvalue_2 (Rendering|Material|CreateDynamicMaterialInstance (Variables|Default|GetStaticMesh) 0 "/MobaMapContent/Maps/MainMapBlockout/Materials/M_BaseWater.M_BaseWater" "None" :!class /Script/Engine.PrimitiveComponent))
  (Variables|Default|SetMID_Water _returnvalue_2)
  (CallFunction|PrepareBaseWater))

(fn PrepareBaseWater
  (Rendering|Material|SetScalarParameterValue (Variables|Default|GetMID_Water) "SimulationDistance" (Variables|Default|GetSimulationDistance) :!class /Script/Engine.MaterialInstanceDynamic)
  (Rendering|Material|SetVectorParameterValue (Variables|Default|GetMID_Water) "NearColor" (Variables|Default|GetNearColor) :!class /Script/Engine.MaterialInstanceDynamic)
  (Rendering|Material|SetVectorParameterValue (Variables|Default|GetMID_Water) "FarColor" (Variables|Default|GetFarColor) :!class /Script/Engine.MaterialInstanceDynamic)
  (Rendering|Material|SetScalarParameterValue (Variables|Default|GetMID_Water) "Opacity" (Variables|Default|GetOpacity) :!class /Script/Engine.MaterialInstanceDynamic)
  (Rendering|Material|SetScalarParameterValue (Variables|Default|GetMID_Water) "Depth" (Variables|Default|GetDepth) :!class /Script/Engine.MaterialInstanceDynamic)
  (Rendering|Material|SetScalarParameterValue (Variables|Default|GetMID_Water) "Waterline" (Variables|Default|GetWaterline) :!class /Script/Engine.MaterialInstanceDynamic)
  (Rendering|Material|SetScalarParameterValue (Variables|Default|GetMID_Water) "Refraction" (Variables|Default|GetRefraction) :!class /Script/Engine.MaterialInstanceDynamic)
  (Utilities|IsValid (Variables|Default|GetMID_HeightSimulation)
    (:Is%20Valid
      (Utilities|IsValid (Variables|Default|GetMID_ComputeNormals)
        (:Is%20Valid
          (Rendering|Material|SetScalarParameterValue (Variables|Default|GetMID_HeightSimulation) "Dampening" (Variables|Default|GetDampening) :!class /Script/Engine.MaterialInstanceDynamic)
          (Rendering|Material|SetScalarParameterValue (Variables|Default|GetMID_HeightSimulation) "WaveSpeed" (Variables|Default|GetWaveSpeed) :!class /Script/Engine.MaterialInstanceDynamic)
          (Rendering|Material|SetScalarParameterValue (Variables|Default|GetMID_HeightSimulation) "TexelSize" (Variables|Default|GetTexelSize) :!class /Script/Engine.MaterialInstanceDynamic)
          (Rendering|Material|SetScalarParameterValue (Variables|Default|GetMID_ComputeNormals) "TexelSize" (Variables|Default|GetTexelSize) :!class /Script/Engine.MaterialInstanceDynamic))))))

(fn PrepareHeightRT
  (params (Size :type Float%20%28double-precision%29))
  (bind _returnvalue (Math|Float|Truncate Size))
  (bind _returnvalue_2 (Math|Float|Truncate Size))
  (bind _returnvalue_3 (Math|Float|Truncate Size))
  (bind _returnvalue_4 (Math|Float|Truncate Size))
  (bind _returnvalue_5 (Rendering|CreateRenderTarget2D _returnvalue_2 _returnvalue_2 "RTF_R16f"))
  (Variables|Default|SetRT_Height_00 _returnvalue_5)
  (bind _returnvalue_6 (Rendering|CreateRenderTarget2D _returnvalue_3 _returnvalue_3 "RTF_R16f"))
  (Variables|Default|SetRT_Height_01 _returnvalue_6)
  (bind _returnvalue_7 (Rendering|CreateRenderTarget2D _returnvalue_4 _returnvalue_4 "RTF_R16f"))
  (Variables|Default|SetRT_Height_02 _returnvalue_7)
  (bind _returnvalue_8 (Rendering|CreateRenderTarget2D _returnvalue _returnvalue "RTF_RGBA16f"))
  (Variables|Default|SetRT_Height_Normal _returnvalue_8)
  (Rendering|ClearRenderTarget2D (Variables|Default|GetRT_Height_00))
  (Rendering|ClearRenderTarget2D (Variables|Default|GetRT_Height_01))
  (Rendering|ClearRenderTarget2D (Variables|Default|GetRT_Height_02))
  (Rendering|ClearRenderTarget2D (Variables|Default|GetRT_Height_Normal)))

(fn PrepareCaptureRT
  (params (Size :type Float%20%28double-precision%29))
  (bind _returnvalue (Math|Float|Truncate (Variables|Default|GetSize)))
  (bind _returnvalue_2 (Math|Float|Truncate (Variables|Default|GetSize)))
  (bind _returnvalue_3 (Math|Float|Truncate (Variables|Default|GetSize)))
  (bind _returnvalue_4 (Rendering|CreateRenderTarget2D _returnvalue _returnvalue "RTF_R8"))
  (Variables|Default|SetRT_PlayerCapture _returnvalue_4)
  (bind _returnvalue_5 (Rendering|CreateRenderTarget2D _returnvalue_3 _returnvalue_3 "RTF_R8"))
  (Variables|Default|SetRT_RainCapture _returnvalue_5)
  (bind _returnvalue_6 (Rendering|CreateRenderTarget2D _returnvalue_2 _returnvalue_2 "RTF_R8"))
  (Variables|Default|SetRT_ImpactCapture _returnvalue_6))

(fn PrepareSceneCapture
  (Variables|/Script/Engine.SceneCaptureComponent2D|SetTextureTarget (Variables|Default|GetSceneCaptureComponent2D) (Variables|Default|GetRT_PlayerCapture))
  (Variables|/Script/Engine.SceneCaptureComponent2D|SetOrthoWidth (Variables|Default|GetSceneCaptureComponent2D) (Variables|Default|GetSimulationDistance))
  (Variables|/Script/Engine.SceneCaptureComponent2D|SetClipPlaneBase (Variables|Default|GetSceneCaptureComponent2D) (Math|Vector|MakeVector 0.0 0.0 (- (.z (Transformation|GetWorldLocation (Variables|Default|GetStaticMesh))) (Variables|Default|GetSceneCaptureOffset))))
  (Rendering|Material|SetScalarParameterValue (Variables|Default|GetMID_Splat) "SimulationDivisor" (- (Variables|Default|GetSimulationDistance) (Variables|Default|GetRenderTargetResolution)) :!class /Script/Engine.MaterialInstanceDynamic)
  (Rendering|Material|SetScalarParameterValue (Variables|Default|GetMID_Splat) "RenderTargetResolution" (Variables|Default|GetRenderTargetResolution) :!class /Script/Engine.MaterialInstanceDynamic)
  (Rendering|Material|SetTextureParameterValue (Variables|Default|GetMID_Splat) "PlayerCapture" (Variables|Default|GetRT_PlayerCapture))
  (Rendering|Material|SetTextureParameterValue (Variables|Default|GetMID_Splat) "RainCapture" (Variables|Default|GetRT_RainCapture))
  (Rendering|Material|SetTextureParameterValue (Variables|Default|GetMID_Splat) "ImpactCapture" (Variables|Default|GetRT_ImpactCapture))
  (Rendering|Material|SetTextureParameterValue (Variables|Default|GetMID_Water) "HeightNormal" (Variables|Default|GetRT_Height_Normal)))